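; Stimpack health pickup actor that heals the player when they walk into it.
; On sphere overlap with a PlayerCharacter_BP below full health, it adds a small amount of health, clamped to the maximum.
; It then plays a pickup sound, triggers the in-game UI's item pickup feedback and destroys itself, with a DoOnce guarding against repeat triggers.
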(event `self.Sphere.OnComponentBeginOverlap`
  (params (OverlappedComponent :type "PrimitiveComponent Object Reference") (OtherActor :type "Actor Object Reference") (OtherComp :type "PrimitiveComponent Object Reference") (OtherBodyIndex :type Integer) (bFromSweep :type Boolean) (SweepResult :type "HitResult Structure (by ref)"))
  (bind _asplayer_character_bp (cast `/Game/PlayerBlueprints/PlayerCharacter_BP` OtherActor))
  (bind _currenthealth (`/Game/PlayerBlueprints/PlayerCharacter_BP.CurrentHealth` _asplayer_character_bp))
  (if (not (>= _currenthealth 100))
    (`/Engine/EditorBlueprintResources/StandardMacros.DoOnce` false
      (:`Completed`
        (set `/Game/PlayerBlueprints/PlayerCharacter_BP.CurrentHealth` (`KismetMathLibrary.Clamp` (+ _currenthealth 10) 0 100) _asplayer_character_bp)
        (`GameplayStatics.PlaySound2D` "/Game/SFX/Interact/Item/DSITEMUP.DSITEMUP" 1.0 1.0 0.0 null null)
        (`/Game/UI/InGame_UI.ItemPickup` (`/Game/PlayerBlueprints/InGame_PC.In Game UI` (`/Game/PlayerBlueprints/PlayerCharacter_BP.As in Game PC` _asplayer_character_bp)))
        (`self.K2_DestroyActor`)))))

(fn `UserConstructionScript`)