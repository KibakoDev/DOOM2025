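; Base enemy Blueprint that activates when the player overlaps its trigger box, then yaws toward the player and calls Move and FireWeapon, both empty here.
; Point damage reduces health, plays hit montage and sound, and on death ragdolls with an impulse; Zombieman enemies also drop their weapon and a clip.
; A Niagara blood burst exports particle data back to the actor to spawn blood decals.
; Randomized idle sounds can repeat while alive.
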(event `self.ReceiveBeginPlay`
  ; Begin Play
  (bind _asplayer_character_bp (cast `/Game/PlayerBlueprints/PlayerCharacter_BP` (`GameplayStatics.GetPlayerCharacter` 0)))
  (set `self.As Player Character BP` _asplayer_character_bp))

(event `self.ReceiveTick`
  (params (DeltaSeconds :type "Float (single-precision)"))
  (bind (_returnvalue_roll _returnvalue_pitch _returnvalue_yaw) (`KismetMathLibrary.BreakRotator` (`KismetMathLibrary.FindLookAtRotation` (`self.K2_GetActorLocation`) (`self.K2_GetActorLocation` (`GameplayStatics.GetPlayerCharacter` 0)))))
  ; Event Tick
  (if (`self.IsTriggered?`)
    (`self.K2_SetActorRotation` (`KismetMathLibrary.MakeRotator` 0.0 0.0 _returnvalue_yaw))))

(event `self.TriggerBox.OnActorBeginOverlap`
  (params (OverlappedActor :type "Actor Object Reference") (OtherActor :type "Actor Object Reference"))
  ; TriggerBox
  (switch `/Game/EnemiesBlueprints/TriggerMethod_Enum` (`self.TriggerMethod`)
    (:`NewEnumerator1`
      (cast `/Game/PlayerBlueprints/PlayerCharacter_BP` OtherActor)
      (`self.Initialize`))))

(event `Initialize`
  ; Initialize
  (`/Engine/EditorBlueprintResources/StandardMacros.DoOnce` false
    (:`Completed`
      (set `self.IsTriggered?` true)
      (`self.Move`)
      (`self.Play Idle Sound`)
      (`KismetSystemLibrary.Delay` (`KismetMathLibrary.RandomFloatInRange` 0.0 2.0))
      (`self.FireWeapon`))))

(event `Move`
  ; Movement
)

(event `self.ReceiveParticleData`
  (params (Data :type "Array of BasicParticleData Structure (by ref)") (NiagaraSystem :type "NiagaraSystem Object Reference") (SimulationPositionOffset :type "Vector Structure (by ref)"))
  ; Spawn blood decals
  (`/Engine/EditorBlueprintResources/StandardMacros.IsValid` (`self.CurrentBloodParticle`)
    (:`Is Valid`
      (for _array_element Data
        (bind (_position _size _velocity) (break `BasicParticleData` _array_element))
        (`|SpawnActorFromClass` "/Game/FX/BloodFX/Blueprints/BP_Decal.BP_Decal_C" (`KismetMathLibrary.MakeTransform` _position (`KismetMathLibrary.MakeRotFromZY` _velocity (`KismetMathLibrary.Cross_VectorVector` (`KismetMathLibrary.Normal` _velocity) (`KismetMathLibrary.Normal` (- _position (`SceneComponent.K2_GetComponentLocation` (`self.CurrentBloodParticle`)))))) (* (`KismetMathLibrary.MakeVector` (`KismetMathLibrary.RandomFloatInRange` 0.9 1.3) (`KismetMathLibrary.RandomFloatInRange` 0.9 1.3) (`KismetMathLibrary.RandomFloatInRange` 0.9 1.3)) 3.0)) "Undefined" "MultiplyWithRoot" null 0.0 1.0 10000.0 "/Game/FX/BloodFX/Materials/pixelated/MI_BloodDecal_Pix.MI_BloodDecal_Pix" _size false true null)))))

(event `Play Idle Sound`
  ; Sounds
  (`KismetSystemLibrary.Delay` (`KismetMathLibrary.RandomFloatInRange` 0.0 2.0))
  (if (and (`KismetMathLibrary.RandomBool`) (> (`self.CurrentHealth`) 0) (`self.IsTriggered?`))
    (`GameplayStatics.SpawnSoundAttached` (`self.Idle Sounds`) (`self.Mesh`) "None" (0.0 0.0 0.0) (struct) "KeepRelativeOffset" false 1.0 1.0 0.0 null null)
    (`KismetSystemLibrary.Delay` (`KismetMathLibrary.RandomFloatInRange` 2.0 5.0))
    (`self.Play Idle Sound`)))

(event `Play Damaged Sound`
  ; Sounds
  (`/Engine/EditorBlueprintResources/StandardMacros.DoOnce` false :!label _label
    (:`Completed`
      (`|ExecutionSequence`
        (:`then_0`
          (`GameplayStatics.SpawnSoundAttached` (`self.Damaged Sounds`) (`self.Mesh`) "None" (0.0 0.0 0.0) (struct) "KeepRelativeOffset" false 1.0 1.0 0.0 null null))
        (:`then_1`
          (`KismetSystemLibrary.Delay` 0.5)
          (goto _label :!via `Reset`))))))

(event `self.ReceivePointDamage`
  (params (Damage :type "Float (single-precision)") (DamageType :type "DamageType Object Reference") (HitLocation :type "Vector Structure") (HitNormal :type "Vector Structure") (HitComponent :type "PrimitiveComponent Object Reference") (BoneName :type Name) (ShotFromDirection :type "Vector Structure") (InstigatedBy :type "Controller Object Reference") (DamageCauser :type "Actor Object Reference") (HitInfo :type "HitResult Structure (by ref)"))
  (bind _mesh (`self.Mesh`))
  ; Event Damage
  (if (> (`self.CurrentHealth`) 0)
    (bind _output_get (set `self.CurrentHealth` (`KismetMathLibrary.Clamp` (- (`self.CurrentHealth`) (`KismetMathLibrary.FTrunc` Damage)) 0 (`self.MaxHealth`))))
    (if (not (> _output_get 0))
      (`/Engine/EditorBlueprintResources/StandardMacros.DoOnce` false
        (:`Completed`
          (`PrimitiveComponent.SetCollisionEnabled` (`self.CapsuleComponent`) "NoCollision")
          (`PrimitiveComponent.SetCollisionEnabled` _mesh "QueryAndPhysics")
          (`PrimitiveComponent.SetSimulatePhysics` _mesh true)
          (`PrimitiveComponent.AddImpulse` _mesh (* HitNormal -500.0) BoneName true)
          (bind _aszombieman_enemy_bp (cast `/Game/EnemiesBlueprints/Zombieman/Zombieman_Enemy_BP` self)
            (:`then`
              (bind _weapon (`/Game/EnemiesBlueprints/Zombieman/Zombieman_Enemy_BP.Weapon` _aszombieman_enemy_bp))
              (`PrimitiveComponent.SetCollisionEnabled` _weapon "QueryAndPhysics")
              (`PrimitiveComponent.SetSimulatePhysics` _weapon true)
              (`|SpawnActorFromClass` "/Game/InteractBlueprints/Clip/Clip_BP.Clip_BP_C" (`KismetMathLibrary.MakeTransform` (`SceneComponent.K2_GetComponentLocation` (`self.Mesh`))) "Undefined" "MultiplyWithRoot" null null))
            (:`CastFailed`
              _)))))
    (`self.PlayAnimMontage` "/Game/EnemiesBlueprints/Zombieman/Mesh/Animations/Rifle_Hit_Montage.Rifle_Hit_Montage")
    (bind _returnvalue (`NiagaraFunctionLibrary.SpawnSystemAtLocation` "/Game/FX/BloodFX/Particles/P_SplashBurst_Decal_Pix.P_SplashBurst_Decal_Pix" HitLocation (`KismetMathLibrary.Conv_VectorToRotator` HitNormal)))
    (bind _output_get_2 (set `self.CurrentBloodParticle` _returnvalue))
    (`NiagaraComponent.SetNiagaraVariableObject` _output_get_2 "User.Data" self)
    (`self.Play Damaged Sound`)
    (else
      (bind _returnvalue_2 (`NiagaraFunctionLibrary.SpawnSystemAtLocation` "/Game/FX/BloodFX/Particles/P_SplashBurst_Decal_Pix.P_SplashBurst_Decal_Pix" HitLocation (`KismetMathLibrary.Conv_VectorToRotator` HitNormal)))
      (set `self.CurrentBloodParticle` _returnvalue_2))))

(event `FireWeapon`
  ; Fire Weapon
)

(fn `UserConstructionScript`)