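; Imp fireball Actor that deals damage on impact, with a launch sound attached at spawn and a constant spin on the fireball component.
; BeginPlay explicitly sets the collision sphere not to ignore its owner when moving.
; A sphere hit applies random point damage within the AttackDamage range, credited to the owner as damage causer.
; It then spawns an explosion effect and sound at the impact point and destroys itself.
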(event `self.ReceiveBeginPlay`
  (`PrimitiveComponent.IgnoreActorWhenMoving` (`self.Sphere`) (`self.GetOwner`) false)
  (`GameplayStatics.SpawnSoundAttached` "/Game/SFX/Projectiles/Fireball/DSFIRSHT.DSFIRSHT" (`self.Fireball`) "None" (0.0 0.0 0.0) (struct) "KeepRelativeOffset" false 1.0 1.0 0.0 null null))

(event `self.ReceiveTick`
  (params (DeltaSeconds :type "Float (single-precision)"))
  (`SceneComponent.K2_AddLocalRotation` (`self.Fireball`) (struct :`Pitch` 5.0 :`Yaw` 5.0 :`Roll` 5.0) false false))

(event `self.Sphere.OnComponentHit`
  (params (HitComponent :type "PrimitiveComponent Object Reference") (OtherActor :type "Actor Object Reference") (OtherComp :type "PrimitiveComponent Object Reference") (NormalImpulse :type "Vector Structure") (Hit :type "HitResult Structure (by ref)"))
  (bind (_bblockinghit _binitialoverlap _time _distance _location _impactpoint _normal _impactnormal _physmat _hitactor _hitcomponent _hitbonename _bonename _hititem _elementindex _faceindex _tracestart) (`GameplayStatics.BreakHitResult` Hit))
  (bind (_attackdamage_x _attackdamage_y) (break `IntPoint` (`self.AttackDamage`)))
  (`GameplayStatics.ApplyPointDamage` OtherActor (`KismetMathLibrary.Conv_IntToDouble` (`KismetMathLibrary.RandomIntegerInRange` _attackdamage_x _attackdamage_y)) _tracestart Hit null (`self.GetOwner`))
  (`GameplayStatics.SpawnEmitterAtLocation` "/Game/FX/MainFX/P_ky_explosion.P_ky_explosion" _impactpoint (`KismetMathLibrary.Conv_VectorToRotator` _impactnormal) (0.4 0.4 0.4))
  (`GameplayStatics.PlaySoundAtLocation` "/Game/SFX/Projectiles/Fireball/DSFIRXPL.DSFIRXPL" _impactpoint (struct) 1.0 1.0 0.0 null null null null)
  (`self.K2_DestroyActor`))

(fn `UserConstructionScript`)