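; Imp enemy Blueprint that wanders around and throws fireballs at the player once triggered.
; Move picks a random reachable point near the imp and re-calls itself, after a short pause on success or at once on failure.
; FireWeapon plays an attack montage, spawns a fireball from the throw socket aimed at the player, then repeats after a random delay while both are alive.
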(event `self.Move`
  ; Movement
  (if (`self.IsTriggered?`)
    (`|AIMoveTo` self (`NavigationSystemV1.K2_GetRandomReachablePointInRadius` (`self.K2_GetActorLocation`) 500.0 null null) null 5.0 true
      (:`OnSuccess`
        (`KismetSystemLibrary.Delay` 0.75))
      (:`OnFail`
        _))
    (`self.Move`)))

(event `self.FireWeapon`
  (bind (_attackrate_x _attackrate_y) (`KismetMathLibrary.BreakVector2D` (`self.AttackRate`)))
  (bind _returnvalue (`SceneComponent.K2_GetComponentLocation` (`self.Throw_Socket`)))
  ; Fire Weapon
  (if (and (> (`self.CurrentHealth`) 0) (`self.IsTriggered?`) (not (`/Game/PlayerBlueprints/PlayerCharacter_BP.Dead?` (`self.As Player Character BP`))))
    (`self.PlayAnimMontage` "/Game/EnemiesBlueprints/Imp/Mesh/Animations/Wizard_Attack_Montage.Wizard_Attack_Montage")
    (`KismetSystemLibrary.Delay` 0.5)
    (`|SpawnActorFromClass` "/Game/EnemiesBlueprints/Imp/Fireball_BP.Fireball_BP_C" (`KismetMathLibrary.MakeTransform` _returnvalue (`KismetMathLibrary.FindLookAtRotation` _returnvalue (`self.K2_GetActorLocation` (`GameplayStatics.GetPlayerCharacter` 0)))) "Undefined" "MultiplyWithRoot" self null)
    (`KismetSystemLibrary.Delay` (`KismetMathLibrary.RandomFloatInRange` _attackrate_x _attackrate_y))
    (`self.FireWeapon`)))

(fn `UserConstructionScript`
  (`parent.UserConstructionScript`))