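; Zombieman enemy that chases the player, always rotates to face them and plays randomized idle groans.
; Movement reissues AI MoveTo every half second toward the player's location, randomly offset along X or Y for erratic approaches.
; Point damage plays a hit montage, a throttled pain sound and a Niagara blood burst.
; The burst exports particle data back to the Blueprint, which spawns fading pixelated blood decals from it.
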(event `self.ReceiveBeginPlay`
  ; Begin Play
  (`self.Move`)
  (`self.Play Idle Sound`))

(event `self.ReceiveTick`
  (params (DeltaSeconds :type "Float (single-precision)"))
  ; Event Tick
  (`parent.ReceiveTick` DeltaSeconds)
  (`self.K2_SetActorRotation` (`KismetMathLibrary.FindLookAtRotation` (`self.K2_GetActorLocation`) (`self.K2_GetActorLocation` (`GameplayStatics.GetPlayerCharacter` 0)))))

(event `Move`
  (bind _returnvalue (`KismetMathLibrary.RandomBool`))
  (bind _returnvalue_2 (not _returnvalue))
  (bind (_returnvalue_x _returnvalue_y _returnvalue_z) (`KismetMathLibrary.BreakVector` (`self.K2_GetActorLocation` (`GameplayStatics.GetPlayerCharacter` 0))))
  (bind _returnvalue_3 (`KismetMathLibrary.SelectFloat` 500.0 -500.0 _returnvalue_2))
  ; Movement
  (`|AIMoveTo` self (`KismetMathLibrary.MakeVector` (select `bool` _returnvalue :`false` _returnvalue_x :`true` (+ _returnvalue_x _returnvalue_3)) (select `bool` _returnvalue_2 :`false` _returnvalue_y :`true` (+ _returnvalue_y _returnvalue_3)) _returnvalue_z) null 5.0 true
    (:`then`
      (`KismetSystemLibrary.Delay` 0.5)
      (`self.Move`))))

(event `Play Idle Sound`
  ; Sounds
  (`KismetSystemLibrary.Delay` (`KismetMathLibrary.RandomFloatInRange` 3.0 7.0))
  (if (`KismetMathLibrary.RandomBool`)
    (`GameplayStatics.SpawnSoundAttached` "/Game/SFX/Ennemies/Idle/Monster_Idle_Cue.Monster_Idle_Cue" (`self.Mesh`) "None" (0.0 0.0 0.0) (struct) "KeepRelativeOffset" false 1.0 1.0 0.0 null null)
    (`self.Play Idle Sound`)))

(event `Play Damaged Sound`
  ; Sounds
  (`/Engine/EditorBlueprintResources/StandardMacros.DoOnce` false :!label _label
    (:`Completed`
      (`|ExecutionSequence`
        (:`then_0`
          (`GameplayStatics.SpawnSoundAttached` "/Game/SFX/Ennemies/Damaged/Monster_Damaged_Cue.Monster_Damaged_Cue" (`self.Mesh`) "None" (0.0 0.0 0.0) (struct) "KeepRelativeOffset" false 1.0 1.0 0.0 null null))
        (:`then_1`
          (`KismetSystemLibrary.Delay` 0.5)
          (goto _label :!via `Reset`))))))

(event `self.ReceivePointDamage`
  (params (Damage :type "Float (single-precision)") (DamageType :type "DamageType Object Reference") (HitLocation :type "Vector Structure") (HitNormal :type "Vector Structure") (HitComponent :type "PrimitiveComponent Object Reference") (BoneName :type Name) (ShotFromDirection :type "Vector Structure") (InstigatedBy :type "Controller Object Reference") (DamageCauser :type "Actor Object Reference") (HitInfo :type "HitResult Structure (by ref)"))
  ; Event Damage
  (`self.PlayAnimMontage` "/Game/EnemiesBlueprints/Zombieman/Mesh/Animations/Zombieman_AnimMontage_Hit.Zombieman_AnimMontage_Hit")
  (bind _returnvalue (`NiagaraFunctionLibrary.SpawnSystemAtLocation` "/Game/FX/BloodFX/Particles/P_SplashBurst_Decal_Pix.P_SplashBurst_Decal_Pix" HitLocation (`KismetMathLibrary.Conv_VectorToRotator` HitNormal)))
  (bind _output_get (set `self.CurrentBloodParticle` _returnvalue))
  (`NiagaraComponent.SetNiagaraVariableObject` _output_get "User.Data" self)
  (`self.Play Damaged Sound`))

(event `self.ReceiveParticleData`
  (params (Data :type "Array of BasicParticleData Structure (by ref)") (NiagaraSystem :type "NiagaraSystem Object Reference") (SimulationPositionOffset :type "Vector Structure (by ref)"))
  ; Spawn blood decals
  (`/Engine/EditorBlueprintResources/StandardMacros.IsValid` (`self.CurrentBloodParticle`)
    (:`Is Valid`
      (for _array_element Data
        (bind (_position _size _velocity) (break `BasicParticleData` _array_element))
        (`|SpawnActorFromClass` "/Game/FX/BloodFX/Blueprints/BP_Decal.BP_Decal_C" (`KismetMathLibrary.MakeTransform` _position (`KismetMathLibrary.MakeRotFromZY` _velocity (`KismetMathLibrary.Cross_VectorVector` (`KismetMathLibrary.Normal` _velocity) (`KismetMathLibrary.Normal` (- _position (`SceneComponent.K2_GetComponentLocation` (`self.CurrentBloodParticle`)))))) (* (`KismetMathLibrary.MakeVector` (`KismetMathLibrary.RandomFloatInRange` 0.9 1.3) (`KismetMathLibrary.RandomFloatInRange` 0.9 1.3) (`KismetMathLibrary.RandomFloatInRange` 0.9 1.3)) 2.0)) "Undefined" "MultiplyWithRoot" null 0.0 1.0 100.0 "/Game/FX/BloodFX/Materials/pixelated/MI_BloodDecal_Pix.MI_BloodDecal_Pix" _size false true null)))))

(fn `UserConstructionScript`
  (`parent.UserConstructionScript`))