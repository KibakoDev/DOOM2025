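; Doom-style sliding door that the player opens as an interact item, with a Rusty flag choosing its material.
; A timeline moves the mesh along Z, then reverses after a delay, polling each tick until the player leaves the box collision.
; The box also sets and clears the player's current interact item.
; On BeginPlay it collects enemies set to trigger on this door and initializes them whenever it opens.
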(event `self.ReceiveBeginPlay`
  ; Begin Play
  (bind _outactors (`GameplayStatics.GetAllActorsOfClass` "/Game/EnemiesBlueprints/Main_Enemy_BP.Main_Enemy_BP_C"))
  (for _array_element _outactors
    (bind _door (`/Game/EnemiesBlueprints/Main_Enemy_BP.Door` _array_element))
    (`/Engine/EditorBlueprintResources/StandardMacros.IsValid` _door
      (:`Is Valid`
        (switch `/Game/EnemiesBlueprints/TriggerMethod_Enum` (`/Game/EnemiesBlueprints/Main_Enemy_BP.TriggerMethod` _array_element)
          (:`NewEnumerator2`
            (if (== _door self)
              (`KismetArrayLibrary.Array_Add` (`self.EnemyList`) _array_element))))))))

(event `Open Door`
  ; Open/Close Door
  (if (not (`self.Opened?`))
    (set `self.Opened?` true)
    (`GameplayStatics.PlaySoundAtLocation` "/Game/SFX/Interact/Door/DSDOROPN.DSDOROPN" (`SceneComponent.K2_GetComponentLocation` (`self.DoorMesh`)) (struct) 1.0 1.0 0.0 null null null null)
    (`|ExecutionSequence`
      (:`then_0`
        (bind (_direction _z) (`Timeline|Open/Close Anim` :!label _label)
          (:`Update`
            (`SceneComponent.K2_SetRelativeLocation` (`self.DoorMesh`) (`KismetMathLibrary.MakeVector` 0.0 0.0 _z) false false))
          (:`Finished`
            (`KismetSystemLibrary.Delay` 5.0)
            (`self.Close Door`))))
      (:`then_1`
        (for _array_element (`self.EnemyList`)
          (`/Engine/EditorBlueprintResources/StandardMacros.IsValid` _array_element
            (:`Is Valid`
              (`/Game/EnemiesBlueprints/Main_Enemy_BP.Initialize` _array_element))))))))

(event `Close Door`
  ; Open/Close Door
  (if (`self.Opened?`)
    (if (`PrimitiveComponent.IsOverlappingActor` (`self.BoxCollision`) (`GameplayStatics.GetPlayerCharacter` 0)) :!label _label_2
      (`KismetSystemLibrary.DelayUntilNextTick`)
      (goto _label_2)
      (else
        (set `self.Opened?` false)
        (`GameplayStatics.PlaySoundAtLocation` "/Game/SFX/Interact/Door/DSDORCLS.DSDORCLS" (`SceneComponent.K2_GetComponentLocation` (`self.DoorMesh`)) (struct) 1.0 1.0 0.0 null null null null)
        (goto _label :!via `Reverse`)))))

(event `self.BoxCollision.OnComponentBeginOverlap`
  (params (OverlappedComponent :type "PrimitiveComponent Object Reference") (OtherActor :type "Actor Object Reference") (OtherComp :type "PrimitiveComponent Object Reference") (OtherBodyIndex :type Integer) (bFromSweep :type Boolean) (SweepResult :type "HitResult Structure (by ref)"))
  ; Overlap Events
  (bind _asplayer_character_bp (cast `/Game/PlayerBlueprints/PlayerCharacter_BP` OtherActor))
  (set `/Game/PlayerBlueprints/PlayerCharacter_BP.CurrentInteractItem` self _asplayer_character_bp))

(event `self.BoxCollision.OnComponentEndOverlap`
  (params (OverlappedComponent :type "PrimitiveComponent Object Reference") (OtherActor :type "Actor Object Reference") (OtherComp :type "PrimitiveComponent Object Reference") (OtherBodyIndex :type Integer))
  ; Overlap Events
  (bind _asplayer_character_bp (cast `/Game/PlayerBlueprints/PlayerCharacter_BP` OtherActor))
  (set `/Game/PlayerBlueprints/PlayerCharacter_BP.CurrentInteractItem` null _asplayer_character_bp))

(fn `UserConstructionScript`
  (`PrimitiveComponent.SetMaterial` (`self.DoorMesh`) 0 (select `bool` (`self.Rusty?`) :`false` "/Game/Maps/Mesh/Materials/BIGDOOR21.BIGDOOR21" :`true` "/Game/Maps/Mesh/Materials/BIGDOOR41.BIGDOOR41" :!type "MaterialInterface Object Reference")))