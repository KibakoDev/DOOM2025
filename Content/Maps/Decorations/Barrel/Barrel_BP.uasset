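; Explosive barrel decoration that loses one Health per point damage hit and explodes when it reaches zero.
; Radial damage skips the health count and triggers the same explosion after a short delay, so nearby barrels can chain-react.
; The explosion, guarded by a DoOnce, applies radial damage with falloff, spawns an emitter and sound, then destroys the actor.
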(event `self.ReceivePointDamage`
  (params (Damage :type "Float (single-precision)") (DamageType :type "DamageType Object Reference") (HitLocation :type "Vector Structure") (HitNormal :type "Vector Structure") (HitComponent :type "PrimitiveComponent Object Reference") (BoneName :type Name) (ShotFromDirection :type "Vector Structure") (InstigatedBy :type "Controller Object Reference") (DamageCauser :type "Actor Object Reference") (HitInfo :type "HitResult Structure (by ref)"))
  (bind _returnvalue (`SceneComponent.K2_GetComponentLocation` (`self.BarrelMesh`)))
  (if (> (`self.Health`) 0)
    (bind _output_get (set `self.Health` (`KismetMathLibrary.Clamp` (- (`self.Health`) 1) 0 2)))
    (if (not (> _output_get 0))
      (`/Engine/EditorBlueprintResources/StandardMacros.DoOnce` false :!label _label
        (:`Completed`
          (set `self.Health` 0)
          (`GameplayStatics.ApplyRadialDamageWithFalloff` :`BaseDamage` 50.0 :`MinimumDamage` 5.0 :`Origin` (`self.K2_GetActorLocation`) :`DamageInnerRadius` 20.0 :`DamageOuterRadius` 500.0 :`DamageFalloff` 2.0 :`DamageCauser` self :`InstigatedByController` null)
          (`GameplayStatics.SpawnEmitterAtLocation` "/Game/FX/MainFX/P_ky_explosion.P_ky_explosion" _returnvalue (struct) (0.5 0.5 0.5))
          (`GameplayStatics.PlaySoundAtLocation` "/Game/SFX/Projectiles/Fireball/DSFIRXPL.DSFIRXPL" _returnvalue (struct) 1.0 1.0 0.0 null null null null)
          (`self.K2_DestroyActor`))))))

(event `self.ReceiveRadialDamage`
  (params (DamageReceived :type "Float (single-precision)") (DamageType :type "DamageType Object Reference") (Origin :type "Vector Structure") (HitInfo :type "HitResult Structure (by ref)") (InstigatedBy :type "Controller Object Reference") (DamageCauser :type "Actor Object Reference"))
  (`KismetSystemLibrary.Delay` 0.2)
  (goto _label))

(fn `UserConstructionScript`)